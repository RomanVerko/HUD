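; BP_Shape is a falling collectible shape that the player catches for points.
; Tick moves it down at FallSpeed with a swept world offset.
; On overlap with BP_Player it destroys itself, then compares its Material to the color materials to increment that color's GameManager counter and pick a point value.
; Red subtracts points, the other colors add them, and GameManager receives the result through IncrementShapesCollected.
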(event `self.ReceiveTick`
  (params (DeltaSeconds :type "Float (single-precision)"))
  (`self.K2_AddActorWorldOffset` (`KismetMathLibrary.MakeVector` 0.0 0.0 (* (* DeltaSeconds (`self.FallSpeed`)) -1.0)) true))

(event `self.ReceiveActorBeginOverlap`
  (params (OtherActor :type "Actor Object Reference"))
  (bind _material (`self.Material`))
  (bind _gamemanager (`self.GameManager`))
  ;[1 1 1] Destroing actors
  (cast `/Game/GeometryCatcher/Blueprints/BP_Player` OtherActor)
  (`self.K2_DestroyActor`)
  ;[1 1 1] Changing the sum of figures of each color
  (if (== _material (`self.RedMaterial`))
    (`/Game/GeometryCatcher/Blueprints/BP_GameManager.IncrementRedShapesCollected` _gamemanager)
    (set `self.AddPoins` -3)
    (elif (== _material (`self.GreenMaterial`))
      (`/Game/GeometryCatcher/Blueprints/BP_GameManager.IncrementGreenShapesCollected` _gamemanager)
      (set `self.AddPoins` 6)
      (elif (== _material (`self.BlueMaterial`))
        (`/Game/GeometryCatcher/Blueprints/BP_GameManager.IncrementBlueShapesCollected` _gamemanager)
        (set `self.AddPoins` 3)
        (elif (== _material (`self.PurpleMaterial`))
          (`/Game/GeometryCatcher/Blueprints/BP_GameManager.IncrementPurpleShapesCollected` _gamemanager)
          (set `self.AddPoins` 5)
          (else
            (`/Game/GeometryCatcher/Blueprints/BP_GameManager.IncrementOrangeShapesCollected` _gamemanager)
            (set `self.AddPoins` 4))))))
  (`/Game/GeometryCatcher/Blueprints/BP_GameManager.IncrementShapesCollected` (`self.GameManager`) (`self.AddPoins`)))

(fn `UserConstructionScript`)